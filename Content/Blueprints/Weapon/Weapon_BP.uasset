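; Player rifle actor (RU74) that handles automatic fire, recoil, ammo and reloading.
; A looping timer fires Shooting, which plays arm and gun montages and spawns Bullet_BP from the muzzle socket within a spread cone that tightens when aiming.
; Each shot runs a timeline that kicks controller yaw and pitch.
; Reload zeroes the magazine, plays empty or partial montages, then refills it from reserve ammo on completion.
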(event `self.ReceiveBeginPlay`
  (bind _asplayer_bp (cast `/Game/Blueprints/Character/Player_BP` (`GameplayStatics.GetPlayerPawn` 0)))
  (set `self.As Player BP` _asplayer_bp))

(event `Shooting`
  (bind (_return_value_location _returnvalue) (`self.AmmoShotChange`))
  (bind _as_player_anim (`/Game/Blueprints/Character/Player_BP.As Player Anim` (`self.As Player BP`)))
  (if (<= (`self.CurrentAmmo`) 0)
    (`GameplayStatics.PlaySound2D` "/Game/Sounds/Weapon/AK74/gun_rifle_dry_fire_01_Cue.gun_rifle_dry_fire_01_Cue" 1.0 1.0 0.0 null null)
    (`KismetSystemLibrary.K2_ClearTimer` null "Shooting")
    (else
      (`AnimInstance.Montage_Play` _as_player_anim (select `bool` (`/Game/Blueprints/Character/Player_Anim.IsAim` _as_player_anim) :`false` "/Game/FPS_Assault_Pack/Animations/RU74/A_Arms_RU74_Shoot01_Montage.A_Arms_RU74_Shoot01_Montage" :`true` "/Game/FPS_Assault_Pack/Animations/RU74/A_Arms_RU74_Isight_Shoot01_Montage.A_Arms_RU74_Isight_Shoot01_Montage" :!type "AnimMontage Object Reference") 1.2 "MontageLength" 0.0 true)
      (`AnimInstance.Montage_Play` (`SkeletalMeshComponent.GetAnimInstance` (`self.SkeletalMesh`)) "/Game/FPS_Assault_Pack/Animations/RU74/A_RU74_Shoot01_Montage.A_RU74_Shoot01_Montage" 2.5 "MontageLength" 0.0 true)
      (`|SpawnActorFromClass` "/Game/Blueprints/Weapon/Bullet_BP.Bullet_BP_C" (`KismetMathLibrary.MakeTransform` _return_value_location _returnvalue (0.2 0.2 0.2)) "AlwaysSpawn" "MultiplyWithRoot" null null)
      (bind _result (`/Engine/EditorBlueprintResources/StandardMacros.DecrementInt` (`self.CurrentAmmo`))
        (:`  `
          (`KismetSystemLibrary.PrintString` (`KismetStringLibrary.Conv_IntToString` _result))
          (`self.RecoilCal`))))))

(event `StartShoot`
  (`KismetSystemLibrary.K2_SetTimer` null "Shooting" 0.12 true)
  (`self.Shooting`))

(event `StopShoot`
  (`KismetSystemLibrary.K2_ClearTimer` null "Shooting"))

(event `BeginReload`
  (if (> (`self.TotalAmmo`) 0)
    (if (not (== (`self.MaxAmmo`) (`self.CurrentAmmo`)))
      (set `self.SaveAmmo` (`self.CurrentAmmo`))
      (set `self.CurrentAmmo` 0)
      (if (not (`self.IsReloading`))
        (set `self.IsReloading` true)
        (if (<= (`self.SaveAmmo`) 0)
          (`|PlayMontage` (`Character.Mesh` (`self.As Player BP`)) "/Game/FPS_Assault_Pack/Animations/RU74/A_Arms_RU74_Reload_Empty_Montage.A_Arms_RU74_Reload_Empty_Montage"
            (:`then`
              (`|PlayMontage` (`self.SkeletalMesh`) "/Game/FPS_Assault_Pack/Animations/RU74/A_RU74_Reload_Empty_Montage.A_RU74_Reload_Empty_Montage"
                (:`OnCompleted`
                  _))))
          (else
            (`|PlayMontage` (`Character.Mesh` (`self.As Player BP`)) "/Game/FPS_Assault_Pack/Animations/RU74/A_Arms_RU74_Reload_Montage.A_Arms_RU74_Reload_Montage"
              (:`then`
                (`|PlayMontage` (`self.SkeletalMesh`) "/Game/FPS_Assault_Pack/Animations/RU74/A_RU74_Reload_Montage.A_RU74_Reload_Montage"
                  (:`OnCompleted`
                    _))))))
        (set `self.IsReloading` false)
        (`self.RemainAmmoCal`)
        (bind _output_get (set `self.CurrentAmmo` (`self.SaveAmmo`)))
        (`KismetSystemLibrary.PrintString` (`KismetStringLibrary.Conv_IntToString` _output_get) true true (struct :`R` 1.0 :`B` 0.007519 :`A` 1.0) 10.0)
        (`KismetSystemLibrary.PrintString` (`KismetStringLibrary.Conv_IntToString` (`self.TotalAmmo`)) true true (struct :`G` 1.0 :`B` 0.117987 :`A` 1.0) 10.0)))))

(event `RecoilCal`
  (bind _returnvalue (`GameplayStatics.GetPlayerPawn` 0))
  (bind (_direction _newtrack_1) (`Timeline|Timeline` :!via `PlayFromStart`)
    (:`Update`
      (`Pawn.AddControllerYawInput` _returnvalue (`KismetMathLibrary.Lerp` -0.1 0.1 _newtrack_1))
      (`Pawn.AddControllerPitchInput` _returnvalue (`KismetMathLibrary.Lerp` 0.0 -0.15 _newtrack_1)))))

(fn `AmmoShotChange`
  (returns (`Return Value Location` :type "Vector Structure") (ReturnValue :type "Rotator Structure"))
  (bind (_returnvalue_location _returnvalue_rotation) (`KismetMathLibrary.BreakTransform` (`SceneComponent.GetSocketTransform` (`self.SkeletalMesh`) "b_MuzzleSocket" "RTS_World")))
  (return _returnvalue_location (`KismetMathLibrary.Conv_VectorToRotator` (`KismetMathLibrary.RandomUnitVectorInConeInDegrees` (`KismetMathLibrary.Conv_RotatorToVector` _returnvalue_rotation) (`KismetMathLibrary.SelectFloat` 2.0 4.0 (`/Game/Blueprints/Character/Player_Anim.IsAim` (`/Game/Blueprints/Character/Player_BP.As Player Anim` (`self.As Player BP`))))))))

(fn `RemainAmmoCal`
  (bind _returnvalue (- (`self.TotalAmmo`) (- (`self.MaxAmmo`) (`self.SaveAmmo`))))
  (if (> _returnvalue 0)
    (set `self.TotalAmmo` _returnvalue)
    (set `self.SaveAmmo` (`self.MaxAmmo`))
    (else
      (set `self.SaveAmmo` (+ (`self.SaveAmmo`) (`self.TotalAmmo`)))
      (set `self.TotalAmmo` 0))))

(fn `UserConstructionScript`)