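; Zombie enemy character that chases the first player and goes ragdoll when killed.
; BeginPlay randomizes its skeletal mesh, run or sprint speed, and idle animation with start offset via the Zombie_Anim instance.
; A looping timer reissues AIMoveTo toward the player and sets AI focus on them.
; Damage reduces health, playing random hit-react montages until death disables capsule collision, enables mesh physics and zeroes walk speed.
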(event `self.ReceiveBeginPlay`
  (bind _aszombie_anim (cast `/Game/Blueprints/Zombie/Zombie_Anim` (`SkeletalMeshComponent.GetAnimInstance` (`self.Mesh`))))
  (set `self.As Zombie Anim` _aszombie_anim)
  (`KismetSystemLibrary.K2_SetTimer` null "ChasePlayer" 1.0 true)
  (`self.InitSpeed&Anim`)
  (`self.RandomMesh`))

(event `ChasePlayer`
  (bind _returnvalue (`GameplayStatics.GetPlayerPawn` 0))
  (`|AIMoveTo` self (0.0 0.0 0.0) _returnvalue 100.0
    (:`then`
      (`AIController.K2_SetFocus` (`AIBlueprintHelperLibrary.GetAIController` self) _returnvalue))))

(event `self.ReceiveAnyDamage`
  (params (Damage :type "Float (single-precision)") (DamageType :type "DamageType Object Reference") (InstigatedBy :type "Controller Object Reference") (DamageCauser :type "Actor Object Reference"))
  (bind _mesh (`self.Mesh`))
  (bind _output_get (set `self.Health` (- (`self.Health`) Damage)))
  (if (<= _output_get 0.0)
    (`/Engine/EditorBlueprintResources/StandardMacros.DoOnce` false
      (:`Completed`
        (`PrimitiveComponent.SetCollisionEnabled` (`self.CapsuleComponent`) "NoCollision")
        (`PrimitiveComponent.SetSimulatePhysics` _mesh true)
        (`SkeletalMeshComponent.PlayAnimation` _mesh null false)
        (set `CharacterMovementComponent.MaxWalkSpeed` 0.0 (`self.CharacterMovement`))))
    (elif (not (`self.IsBacking`))
      (set `self.IsBacking` true)
      (`|PlayMontage` (`self.Mesh`) (select `int` (`KismetMathLibrary.RandomIntegerInRange` 0 2) :`0` "/Game/ShirtlessZombiesPack/Zombie_Pack/Animations/InPlace/Hits/Zombie_HitReact_Head_Montage.Zombie_HitReact_Head_Montage" :`1` "/Game/ShirtlessZombiesPack/Zombie_Pack/Animations/InPlace/Hits/Zombie_HitReact_LeftArm_Montage.Zombie_HitReact_LeftArm_Montage" :`2` "/Game/ShirtlessZombiesPack/Zombie_Pack/Animations/InPlace/Hits/Zombie_HitReact_RightArm_Montage.Zombie_HitReact_RightArm_Montage" :!type "AnimMontage Object Reference") 1.3
        (:`OnCompleted`
          _)
        (:`OnInterrupted`
          _))
      (set `self.IsBacking` false))))

(fn `InitSpeed&Anim`
  (bind _as_zombie_anim (`self.As Zombie Anim`))
  (switch `int` (`KismetMathLibrary.RandomIntegerInRange` 0 1)
    (:`0`
      (set `/Game/Blueprints/Zombie/Zombie_Anim.MoveAnim` "/Game/ShirtlessZombiesPack/Zombie_Pack/Animations/InPlace/Locomotion/IP_Run_Front.IP_Run_Front" _as_zombie_anim)
      (set `self.InitSpeed` 200.0))
    (:`1`
      (set `/Game/Blueprints/Zombie/Zombie_Anim.MoveAnim` "/Game/ShirtlessZombiesPack/Zombie_Pack/Animations/InPlace/Locomotion/IP_Sprint_Front.IP_Sprint_Front" _as_zombie_anim)
      (set `self.InitSpeed` 400.0)))
  (set `/Game/Blueprints/Zombie/Zombie_Anim.IdleAnim` (select `int` (`KismetMathLibrary.RandomIntegerInRange` 0 2) :`0` "/Game/ShirtlessZombiesPack/Zombie_Pack/Animations/InPlace/Idle/IP_Idle_01.IP_Idle_01" :`1` "/Game/ShirtlessZombiesPack/Zombie_Pack/Animations/InPlace/Idle/IP_Idle_02.IP_Idle_02" :`2` "/Game/ShirtlessZombiesPack/Zombie_Pack/Animations/InPlace/Idle/IP_Idle_08.IP_Idle_08" :!type "AnimSequenceBase Object Reference") _as_zombie_anim)
  (set `/Game/Blueprints/Zombie/Zombie_Anim.Start Position` (`KismetMathLibrary.RandomFloatInRange` 0.0 1.0) (`self.As Zombie Anim`))
  (set `CharacterMovementComponent.MaxWalkSpeed` (`self.InitSpeed`) (`self.CharacterMovement`)))

(fn `RandomMesh`
  (`SkeletalMeshComponent.SetSkeletalMeshAsset` (`self.Mesh`) (select `int` (`KismetMathLibrary.RandomIntegerInRange` 0 4) :`0` "/Game/ShirtlessZombiesPack/UE4/SK_ZombieBB_V1.SK_ZombieBB_V1" :`1` "/Game/ShirtlessZombiesPack/UE4/SK_ZombieBB_V2.SK_ZombieBB_V2" :`2` "/Game/ShirtlessZombiesPack/UE4/SK_ZombieBB_V3.SK_ZombieBB_V3" :`3` "/Game/ShirtlessZombiesPack/UE4/SK_ZombieBB_V4.SK_ZombieBB_V4" :`4` "/Game/ShirtlessZombiesPack/UE4/SK_ZombieBB_V5.SK_ZombieBB_V5" :!type "SkeletalMesh Object Reference")))

(fn `UserConstructionScript`)